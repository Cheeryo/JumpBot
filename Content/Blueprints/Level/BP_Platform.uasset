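; BP_Platform is a level platform whose PlatformType selects looping movement, hit-activated movement, random placement or temporary disappearance.
; BeginPlay scales timeline play rates from distance and MovingSpeed, then starts the loop or randomly places the Cube between its origin and EndPosition.
; Player-tagged hits alternately play and reverse the activation timeline, or briefly hide the Cube and disable its collision.
; Box overlaps toggle the character's PlayerOnMovingObject flag, auto-clearing it after a short delay.
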(event OnComponentHit(Cube)
  (params (HitComponent :type Primitive%20Component%20Object%20Reference) (OtherActor :type Actor%20Object%20Reference) (OtherComp :type Primitive%20Component%20Object%20Reference) (NormalImpulse :type Vector :default "0, 0, 0") (Hit :type Hit%20Result%20Structure%20%28by%20ref%29))
  (bind _cube (Variables|Default|GetCube))
  (bind _cube_2 (Variables|Default|GetCube))
  (if (Actor|ActorHasTag OtherActor "Player")
    (switch Utilities|FlowControl|Switch|SwitchonEnum_platformType (Variables|Default|GetPlatformType)
      (:NewEnumerator3
        (Utilities|FlowControl|FlipFlop
          (:A
            (bind _newtrack_0 (Timeline|Timeline_Activation PlayFromStart)
              (:Update
                (Transformation|SetRelativeLocation (Variables|Default|GetCube) (Math|Vector|Lerp(Vector) "0, 0, 0" (Variables|Default|GetEndPosition) _newtrack_0) false false))))
          (:B
            (Timeline|Timeline_Activation ReverseFromEnd))))
      (:NewEnumerator2
        (Utilities|FlowControl|Delay 1.0)
        (Rendering|SetVisibility _cube_2 false false)
        (Collision|SetCollisionEnabled _cube_2 "NoCollision")
        (Utilities|FlowControl|Delay 5.0)
        (Rendering|SetVisibility _cube true false)
        (Collision|SetCollisionEnabled _cube "QueryAndPhysics")))))

(event OnComponentBeginOverlap(Box)
  (params (OverlappedComponent :type Primitive%20Component%20Object%20Reference) (OtherActor :type Actor%20Object%20Reference) (OtherComp :type Primitive%20Component%20Object%20Reference) (OtherBodyIndex :type Integer) (bFromSweep :type Boolean) (SweepResult :type Hit%20Result%20Structure%20%28by%20ref%29))
  (if (Utilities|IsValid OtherActor)
    (bind _asbp_third_person_character (Utilities|Casting|CastToBP_ThirdPersonCharacter OtherActor))
    (Variables|/Game/Characters/JumpBot/BP_ThirdPersonCharacter.BP_ThirdPersonCharacter_C|SetPlayerOnMovingObject _asbp_third_person_character true)
    (Utilities|FlowControl|Delay 0.5)
    (Variables|/Game/Characters/JumpBot/BP_ThirdPersonCharacter.BP_ThirdPersonCharacter_C|SetPlayerOnMovingObject _asbp_third_person_character false)))

(event OnComponentEndOverlap(Box)
  (params (OverlappedComponent :type Primitive%20Component%20Object%20Reference) (OtherActor :type Actor%20Object%20Reference) (OtherComp :type Primitive%20Component%20Object%20Reference) (OtherBodyIndex :type Integer))
  (if (Utilities|IsValid OtherActor)
    (bind _asbp_third_person_character (Utilities|Casting|CastToBP_ThirdPersonCharacter OtherActor))
    (Variables|/Game/Characters/JumpBot/BP_ThirdPersonCharacter.BP_ThirdPersonCharacter_C|SetPlayerOnMovingObject _asbp_third_person_character false)))

(event EventBeginPlay
  (bind _endposition (Variables|Default|GetEndPosition))
  (bind _defaultsceneroot (Variables|Default|GetDefaultSceneRoot))
  (bind _returnvalue (Transformation|GetWorldLocation _defaultsceneroot))
  (bind _returnvalue_2 (- _endposition _returnvalue))
  (bind _returnvalue_3 (Math|Vector|VectorLength _returnvalue_2))
  (Components|Timeline|SetPlayRate (Variables|Default|GetTimeline_Moving%20Loop) (/ 1.0 (/ _returnvalue_3 (* (Variables|Default|GetMovingSpeed) 1e+01))))
  (Components|Timeline|SetPlayRate (Variables|Default|GetTimeline_Activation) (/ 1.0 (/ _returnvalue_3 (* (Variables|Default|GetMovingSpeed) 2e+01))))
  (switch Utilities|FlowControl|Switch|SwitchonEnum_platformType (Variables|Default|GetPlatformType)
    (:NewEnumerator0
      (bind _newtrack_0 (Timeline|Timeline_Moving%20Loop PlayFromStart)
        (:Update
          (Transformation|SetRelativeLocation (Variables|Default|GetCube) (Math|Vector|Lerp(Vector) "0, 0, 0" (Variables|Default|GetEndPosition) _newtrack_0) false false))))
    (:NewEnumerator3
      (Variables|Default|SetMovingActivation? true))
    (:NewEnumerator1
      (Transformation|SetRelativeLocation (Variables|Default|GetCube) (Math|Vector|Lerp(Vector) "0, 0, 0" (Variables|Default|GetEndPosition) (Math|Random|RandomFloat)) false false))
    (:NewEnumerator2
      (Variables|Default|SetDisappearing? true))))

(event Collision|EventActorBeginOverlap
  (params (OtherActor :type Actor%20Object%20Reference)))

(fn ConstructionScript)