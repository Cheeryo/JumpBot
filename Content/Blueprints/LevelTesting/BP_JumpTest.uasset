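; Level-testing actor that visualizes a jump arc in the editor, with no active runtime logic.
; The construction script flattens the Intesnity vector, clamps its length and derives arc distance and apex quadratically from it.
; It shapes and rotates a spline along that vector, labels it with the clamped value and draws a debug circle at the vector's coordinates.
; The Height flag adds a second, raised spline arc.
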(event EventBeginPlay)

(event Collision|EventActorBeginOverlap
  (params (OtherActor :type Actor%20Object%20Reference)))

(event EventTick
  (params (DeltaSeconds :type Float%20%28single-precision%29)))

(fn ConstructionScript
  (bind _spline (Variables|Default|GetSpline))
  (bind _textrender (Variables|Default|GetTextRender))
  (Variables|Default|SetIntesnity (Math|Vector|MakeVector (.x (Variables|Default|GetIntesnity)) (.y (Variables|Default|GetIntesnity)) 0.0))
  (Rendering|Components|TextRender|SetText _textrender (Utilities|Text|ToText(String) (Class|KismetMathLibrary|Round64 (Math|Float|Clamp(Float) (Math|Vector|VectorLength (Variables|Default|GetIntesnity)) 3e+02 1e+03))))
  (Transformation|SetRelativeLocation _textrender (Math|Vector|MakeVector (/ (* (Math|Float|Clamp(Float) (Math|Vector|VectorLength (Variables|Default|GetIntesnity)) 3e+02 1e+03) (* (Math|Float|Clamp(Float) (Math|Vector|VectorLength (Variables|Default|GetIntesnity)) 3e+02 1e+03) 0.00095)) 2.0) -3e+01 (/ (* (Math|Float|Clamp(Float) (Math|Vector|VectorLength (Variables|Default|GetIntesnity)) 3e+02 1e+03) (* (Math|Float|Clamp(Float) (Math|Vector|VectorLength (Variables|Default|GetIntesnity)) 3e+02 1e+03) 0.00095)) 2.0)) false false)
  (Spline|SetLocationatSplinePoint _spline 1 (Math|Vector|MakeVector (/ (* (Math|Float|Clamp(Float) (Math|Vector|VectorLength (Variables|Default|GetIntesnity)) 3e+02 1e+03) (* (Math|Float|Clamp(Float) (Math|Vector|VectorLength (Variables|Default|GetIntesnity)) 3e+02 1e+03) 0.00095)) 2.0) 0.0 (/ (* (Math|Float|Clamp(Float) (Math|Vector|VectorLength (Variables|Default|GetIntesnity)) 3e+02 1e+03) (* (Math|Float|Clamp(Float) (Math|Vector|VectorLength (Variables|Default|GetIntesnity)) 3e+02 1e+03) 0.00109)) 2.0)) "Local" true)
  (Spline|SetLocationatSplinePoint _spline 2 (Math|Vector|MakeVector (* (Math|Float|Clamp(Float) (Math|Vector|VectorLength (Variables|Default|GetIntesnity)) 3e+02 1e+03) (* (Math|Float|Clamp(Float) (Math|Vector|VectorLength (Variables|Default|GetIntesnity)) 3e+02 1e+03) 0.00095)) 0.0 0.0) "Local" true)
  (Spline|SetTangentatSplinePoint _spline 1 (Math|Vector|MakeVector (* (* (Math|Float|Clamp(Float) (Math|Vector|VectorLength (Variables|Default|GetIntesnity)) 3e+02 1e+03) (* (Math|Float|Clamp(Float) (Math|Vector|VectorLength (Variables|Default|GetIntesnity)) 3e+02 1e+03) 0.00109)) 0.8) 0.0 0.0) "Local" true)
  (Transformation|AddRelativeRotation (Variables|Default|GetSpline) (Math|Rotator|MakeRotfromX (Variables|Default|GetIntesnity)) false false)
  (Utilities|FlowControl|Sequence
    (:then_0
      (Rendering|Debug|DrawDebugCircle (+ (Variables|Default|GetIntesnity) "0.000000,0.000000,1.000000") 4e+01 12 "(R=1.000000,G=0.000000,B=0.114957,A=1.000000)" 0.0 1e+02 "0.000000,1.000000,0.000000" "0.000000,0.000000,1.000000"))
    (:then_1
      (if (Variables|Default|GetHeight)
        (bind _returnvalue (AddComponent|AddSplineComponent false))
        (Spline|SetLocationatSplinePoint _returnvalue 0 (Math|Vector|MakeVector 0.0 0.0 85.6) "Local" true)
        (Spline|SetLocationatSplinePoint _returnvalue 1 (Math|Vector|MakeVector (/ (* (Math|Float|Clamp(Float) (Math|Vector|VectorLength (Variables|Default|GetIntesnity)) 3e+02 1e+03) (* (Math|Float|Clamp(Float) (Math|Vector|VectorLength (Variables|Default|GetIntesnity)) 3e+02 1e+03) 0.00095)) 2.0) 0.0 (+ (/ (* (Math|Float|Clamp(Float) (Math|Vector|VectorLength (Variables|Default|GetIntesnity)) 3e+02 1e+03) (* (Math|Float|Clamp(Float) (Math|Vector|VectorLength (Variables|Default|GetIntesnity)) 3e+02 1e+03) 0.00109)) 2.0) 1e+02)) "Local" true)
        (Spline|AddSplinePoint _returnvalue (Math|Vector|MakeVector (* (Math|Float|Clamp(Float) (Math|Vector|VectorLength (Variables|Default|GetIntesnity)) 3e+02 1e+03) (* (Math|Float|Clamp(Float) (Math|Vector|VectorLength (Variables|Default|GetIntesnity)) 3e+02 1e+03) 0.00095)) 0.0 85.6) "Local" true)
        (Spline|SetTangentatSplinePoint _returnvalue 0 (Math|Vector|MakeVector 0.0 0.0 0.0) "Local" true)
        (Spline|SetTangentatSplinePoint _returnvalue 1 (Math|Vector|MakeVector (* (* (Math|Float|Clamp(Float) (Math|Vector|VectorLength (Variables|Default|GetIntesnity)) 3e+02 1e+03) (* (Math|Float|Clamp(Float) (Math|Vector|VectorLength (Variables|Default|GetIntesnity)) 3e+02 1e+03) 0.00109)) 0.8) 0.0 0.0) "Local" true)
        (Spline|SetTangentatSplinePoint _returnvalue 2 (Math|Vector|MakeVector 0.0 0.0 0.0) "Local" true)
        (Transformation|AddRelativeRotation _returnvalue (Math|Rotator|MakeRotfromX (Variables|Default|GetIntesnity)) false false)
        (Class|SplineComponent|SetUnselectedSplineSegmentColor _returnvalue (Variables|Default|GetSegment%20Color))))))