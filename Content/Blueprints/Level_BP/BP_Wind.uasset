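; Wind volume that pushes the JumpBot player while they are falling inside its box.
; Wind follows the root's forward vector, either constant or modulated by a stopping or alternating timeline that also scales the arrow.
; Each tick it applies frame-scaled LaunchCharacter calls from Distance over Time, or pelvis impulses on the mesh when the player is dead.
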(event OnComponentBeginOverlap(Box)
  (params (OverlappedComponent :type Primitive%20Component%20Object%20Reference) (OtherActor :type Actor%20Object%20Reference) (OtherComp :type Primitive%20Component%20Object%20Reference) (OtherBodyIndex :type Integer) (bFromSweep :type Boolean) (SweepResult :type Hit%20Result%20Structure%20%28by%20ref%29))
  (if (Actor|ActorHasTag OtherActor "Player")
    (Variables|Default|SetPlayerIsInside true)))

(event OnComponentEndOverlap(Box)
  (params (OverlappedComponent :type Primitive%20Component%20Object%20Reference) (OtherActor :type Actor%20Object%20Reference) (OtherComp :type Primitive%20Component%20Object%20Reference) (OtherBodyIndex :type Integer))
  (if (Actor|ActorHasTag OtherActor "Player")
    (Variables|Default|SetPlayerIsInside false)))

(event EventBeginPlay
  (bind _timeinterval (Variables|Default|GetTimeInterval))
  (bind _returnvalue (/ 1.0 _timeinterval))
  (bind _asbp_jump_bot_character (Utilities|Casting|CastToBP_JumpBotCharacter (Game|GetPlayerCharacter 0)))
  (Variables|Default|SetAs%20BP%20Third%20Person%20Character _asbp_jump_bot_character)
  (Components|Timeline|SetPlayRate (Variables|Default|GetTimeline%20-%20Stopping) _returnvalue)
  (Components|Timeline|SetPlayRate (Variables|Default|GetTimeline%20-%20Alternating) _returnvalue)
  (if (Variables|Default|GetStopping?)
    (bind _alpha (Timeline|Timeline%20-%20Stopping PlayFromStart)
      (:Update
        (Variables|Default|SetWindVelocity (* (Math|Vector|GetForwardVector (Variables|Default|GetDefaultSceneRoot)) _alpha))
        (Transformation|SetRelativeScale3D (Variables|Default|GetArrow) (Math|Vector|MakeVector _alpha 1.0 1.0))))
    (elif (Variables|Default|GetAlternating)
      (bind _alpha_2 (Timeline|Timeline%20-%20Alternating PlayFromStart)
        (:Update
          (Variables|Default|SetWindVelocity (* (Math|Vector|GetForwardVector (Variables|Default|GetDefaultSceneRoot)) _alpha_2))
          (Transformation|SetRelativeScale3D (Variables|Default|GetArrow) (Math|Vector|MakeVector _alpha_2 1.0 1.0))))
      (else
        (Variables|Default|SetWindVelocity (Math|Vector|GetForwardVector (Variables|Default|GetDefaultSceneRoot)))))))

(event EventTick
  (params (DeltaSeconds :type Float%20%28single-precision%29))
  (bind _as_bp_third_person_character (Variables|Default|GetAs%20BP%20Third%20Person%20Character))
  (Variables|Default|SetDelta%20Seconds DeltaSeconds)
  (if (Variables|Default|GetPlayerIsInside)
    (if (AI|Components|NavMovement|IsFalling (Variables|/Script/Engine.Character|GetCharacterMovement (Variables|Default|GetAs%20BP%20Third%20Person%20Character)))
      (if (Variables|/Game/Characters/JumpBot/BP_JumpBotCharacter.BP_JumpBotCharacter_C|GetisDead? _as_bp_third_person_character)
        (Physics|AddImpulse (Variables|/Script/Engine.Character|GetMesh _as_bp_third_person_character) (* (* (Variables|Default|GetWindVelocity) (* (* (/ (Variables|Default|GetDistance) (Variables|Default|GetTime)) (Variables|Default|GetDelta%20Seconds)) 1e+01)) 4e+01) "pelvis" false)
        (else
          (Character|LaunchCharacter _as_bp_third_person_character (* (Variables|Default|GetWindVelocity) (* (* (/ (Variables|Default|GetDistance) (Variables|Default|GetTime)) (Variables|Default|GetDelta%20Seconds)) 1e+01)) false false))))))

(fn ConstructionScript)