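; Conveyor belt level actor that carries the player's JumpBot character along its forward direction.
; A box trigger flags when the player is on it, and Tick moves them at Distance over Time speed.
; If the character is dead, it teleports the mesh instead of moving the actor.
; A second box adds the belt direction to the character's FeetOffset on entry and subtracts it on exit.
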(event OnComponentBeginOverlap(Box1)
  (params (OverlappedComponent :type Primitive%20Component%20Object%20Reference) (OtherActor :type Actor%20Object%20Reference) (OtherComp :type Primitive%20Component%20Object%20Reference) (OtherBodyIndex :type Integer) (bFromSweep :type Boolean) (SweepResult :type Hit%20Result%20Structure%20%28by%20ref%29))
  (if (and (Utilities|IsValid OtherActor) (Actor|ActorHasTag OtherActor "Player"))
    (Variables|/Game/Characters/JumpBot/BP_JumpBotCharacter.BP_JumpBotCharacter_C|SetFeetOffset (Variables|Default|GetAs%20BP%20Third%20Person%20Character) (+ (Variables|/Game/Characters/JumpBot/BP_JumpBotCharacter.BP_JumpBotCharacter_C|GetFeetOffset (Variables|Default|GetAs%20BP%20Third%20Person%20Character)) (Variables|Default|GetConveyorBeltVelocity)))))

(event OnComponentBeginOverlap(Box)
  (params (OverlappedComponent :type Primitive%20Component%20Object%20Reference) (OtherActor :type Actor%20Object%20Reference) (OtherComp :type Primitive%20Component%20Object%20Reference) (OtherBodyIndex :type Integer) (bFromSweep :type Boolean) (SweepResult :type Hit%20Result%20Structure%20%28by%20ref%29))
  (if (and (Utilities|IsValid OtherActor) (Actor|ActorHasTag OtherActor "Player"))
    (Variables|Default|SetPlayerIsOn true)))

(event OnComponentEndOverlap(Box)
  (params (OverlappedComponent :type Primitive%20Component%20Object%20Reference) (OtherActor :type Actor%20Object%20Reference) (OtherComp :type Primitive%20Component%20Object%20Reference) (OtherBodyIndex :type Integer))
  (if (and (Utilities|IsValid OtherActor) (Actor|ActorHasTag OtherActor "Player"))
    (Variables|Default|SetPlayerIsOn false)))

(event OnComponentEndOverlap(Box1)
  (params (OverlappedComponent :type Primitive%20Component%20Object%20Reference) (OtherActor :type Actor%20Object%20Reference) (OtherComp :type Primitive%20Component%20Object%20Reference) (OtherBodyIndex :type Integer))
  (if (and (Utilities|IsValid OtherActor) (Actor|ActorHasTag OtherActor "Player"))
    (Variables|/Game/Characters/JumpBot/BP_JumpBotCharacter.BP_JumpBotCharacter_C|SetFeetOffset (Variables|Default|GetAs%20BP%20Third%20Person%20Character) (- (Variables|/Game/Characters/JumpBot/BP_JumpBotCharacter.BP_JumpBotCharacter_C|GetFeetOffset (Variables|Default|GetAs%20BP%20Third%20Person%20Character)) (Variables|Default|GetConveyorBeltVelocity)))))

(event EventBeginPlay
  (bind _asbp_jump_bot_character (Utilities|Casting|CastToBP_JumpBotCharacter (Game|GetPlayerCharacter 0)))
  (Variables|Default|SetAs%20BP%20Third%20Person%20Character _asbp_jump_bot_character)
  (Variables|Default|SetConveyorBeltVelocity (Math|Vector|GetForwardVector (Variables|Default|GetDefaultSceneRoot))))

(event EventTick
  (params (DeltaSeconds :type Float%20%28single-precision%29))
  (bind _as_bp_third_person_character (Variables|Default|GetAs%20BP%20Third%20Person%20Character))
  (Variables|Default|SetDelta%20Seconds DeltaSeconds)
  (if (Variables|Default|GetPlayerIsOn)
    (if (Variables|/Game/Characters/JumpBot/BP_JumpBotCharacter.BP_JumpBotCharacter_C|GetisDead? _as_bp_third_person_character)
      (Transformation|AddWorldOffset (Variables|/Script/Engine.Character|GetMesh _as_bp_third_person_character) (* (Variables|Default|GetConveyorBeltVelocity) (* (/ (Variables|Default|GetDistance) (Variables|Default|GetTime)) (Variables|Default|GetDelta%20Seconds))) false true)
      (else
        (Transformation|AddActorWorldOffset _as_bp_third_person_character (* (Variables|Default|GetConveyorBeltVelocity) (* (/ (Variables|Default|GetDistance) (Variables|Default|GetTime)) (Variables|Default|GetDelta%20Seconds))))))))

(fn ConstructionScript)