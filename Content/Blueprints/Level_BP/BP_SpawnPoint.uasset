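; BP_SpawnPoint is a checkpoint actor that stores a respawn transform on BP_JumpBotCharacter.
; Overlapping the Sphere with a Player-tagged actor flags the point as activated, writes its root's world location, slightly raised, and rotation to the character, and prints a confirmation.
; Overlapping the Box repeats that write only if the point is already activated, making it the current spawn point again.
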(event OnComponentBeginOverlap(Sphere)
  (params (OverlappedComponent :type Primitive%20Component%20Object%20Reference) (OtherActor :type Actor%20Object%20Reference) (OtherComp :type Primitive%20Component%20Object%20Reference) (OtherBodyIndex :type Integer) (bFromSweep :type Boolean) (SweepResult :type Hit%20Result%20Structure%20%28by%20ref%29))
  (bind _defaultsceneroot (Variables|Default|GetDefaultSceneRoot))
  (if (and (Utilities|IsValid OtherActor) (Actor|ActorHasTag OtherActor "Player"))
    (Variables|Default|SetsetAsSpawnPoint true)
    (bind _asbp_jump_bot_character (Utilities|Casting|CastToBP_JumpBotCharacter OtherActor))
    (Variables|/Game/Characters/JumpBot/BP_JumpBotCharacter.BP_JumpBotCharacter_C|SetSpawnpointLocation _asbp_jump_bot_character (+ (Transformation|GetWorldLocation _defaultsceneroot) "0.000000,0.000000,44.000000"))
    (Variables|/Game/Characters/JumpBot/BP_JumpBotCharacter.BP_JumpBotCharacter_C|SetSpawnpointRotation _asbp_jump_bot_character (Transformation|GetWorldRotation _defaultsceneroot))
    (Development|PrintString "SPAWN POINT SET")))

(event OnComponentBeginOverlap(Box)
  (params (OverlappedComponent :type Primitive%20Component%20Object%20Reference) (OtherActor :type Actor%20Object%20Reference) (OtherComp :type Primitive%20Component%20Object%20Reference) (OtherBodyIndex :type Integer) (bFromSweep :type Boolean) (SweepResult :type Hit%20Result%20Structure%20%28by%20ref%29))
  (bind _defaultsceneroot (Variables|Default|GetDefaultSceneRoot))
  (if (and (Utilities|IsValid OtherActor) (Actor|ActorHasTag OtherActor "Player"))
    (if (Variables|Default|GetsetAsSpawnPoint)
      (bind _asbp_jump_bot_character (Utilities|Casting|CastToBP_JumpBotCharacter (stale OnComponentBeginOverlap(Sphere) OtherActor)))
      (Variables|/Game/Characters/JumpBot/BP_JumpBotCharacter.BP_JumpBotCharacter_C|SetSpawnpointLocation _asbp_jump_bot_character (+ (Transformation|GetWorldLocation _defaultsceneroot) "0.000000,0.000000,44.000000"))
      (Variables|/Game/Characters/JumpBot/BP_JumpBotCharacter.BP_JumpBotCharacter_C|SetSpawnpointRotation _asbp_jump_bot_character (Transformation|GetWorldRotation _defaultsceneroot))
      (Development|PrintString "SPAWN POINT SET"))))

(event EventBeginPlay)

(event Collision|EventActorBeginOverlap
  (params (OtherActor :type Actor%20Object%20Reference)))

(event EventTick
  (params (DeltaSeconds :type Float%20%28single-precision%29)))

(fn ConstructionScript)